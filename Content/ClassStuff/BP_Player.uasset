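; BP_Player is the player-controlled ship, possessed by player controller 0 on BeginPlay.
; Horizontal and Vertical axes offset the PurpleShipC1 component along Pawn0's forward and up vectors, scaled by Speed and frame time, without sweeping.
; Shoot calls Shoot on the BP_Turret child actor.
; Laser runs an object line trace forward from the turret over LaserLength, with the result unused and no debug drawing.
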(event `self.ReceiveBeginPlay`
  (`Controller.Possess` (`GameplayStatics.GetPlayerController` 0) self))

(event `InputAxis|Horizontal`
  (params (AxisValue :type "Float (single-precision)"))
  (`SceneComponent.K2_AddRelativeLocation` (`self.PurpleShip_C_1`) (* (* AxisValue (`self.Speed`) -1.0 (`GameplayStatics.GetWorldDeltaSeconds`)) (`SceneComponent.GetForwardVector` (`self.Pawn_0`))) false false))

(event `InputAxis|Vertical`
  (params (AxisValue :type "Float (single-precision)"))
  (`SceneComponent.K2_AddRelativeLocation` (`self.PurpleShip_C_1`) (* (* AxisValue (`self.Speed`) (`GameplayStatics.GetWorldDeltaSeconds`)) (`SceneComponent.GetUpVector` (`self.Pawn_0`))) false false))

(event `InputAction|Shoot`
  (params (Key :type "Key Structure"))
  (:`Pressed`
    (bind _asbp_turret (cast `/Game/Models/Balloon/BP_Turret` (`ChildActorComponent.ChildActor` (`self.BP_Turret`))))
    (`/Game/Models/Balloon/BP_Turret.Shoot` _asbp_turret)))

(event `InputAction|Laser`
  (params (Key :type "Key Structure"))
  (bind _bp_turret (`self.BP_Turret`))
  (bind _returnvalue (`SceneComponent.K2_GetComponentLocation` _bp_turret))
  (:`Pressed`
    (`KismetSystemLibrary.LineTraceSingleForObjects` _returnvalue (+ _returnvalue (* (`SceneComponent.GetForwardVector` _bp_turret) (`self.LaserLength`))) (`self.Object Types`))))

(fn `UserConstructionScript`)